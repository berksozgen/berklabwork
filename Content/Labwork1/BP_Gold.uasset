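; BP_Gold is a gold pickup with a random value that adds to the player's gold total.
; On BeginPlay it caches Gamemode1, rolls the value and enlarges the ConeM and ConeL components at higher value tiers.
; Its Interact event adds the value to the Golds count on the game mode, prints the new total and destroys the actor.
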(event EventBeginPlay
  (bind _asgamemode_1 (Utilities|Casting|CastToGamemode1 (Game|GetGameMode)))
  (Variables|Default|SetAs%20Gamemode%201 _asgamemode_1)
  (Variables|Default|SetValue (Math|Random|RandomIntegerinRange 1 99))
  (if (> (Variables|Default|GetValue) 25)
    (Transformation|SetRelativeScale3D (Variables|Default|GetConeM) "1.250000,1.250000,1.250000")
    (if (> (Variables|Default|GetValue) 75)
      (Transformation|SetRelativeScale3D (Variables|Default|GetConeL) "1.500000,1.500000,1.500000"))))

(event Collision|EventActorBeginOverlap
  (params (OtherActor :type Actor%20Object%20Reference)))

(event EventTick
  (params (DeltaSeconds :type Float%20%28single-precision%29)))

(event EventInteract
  (bind _as_gamemode_1 (Variables|Default|GetAs%20Gamemode%201))
  (bind _output_get (Variables|/Game/Labwork1/Gamemode1.Gamemode1_C|SetGolds _as_gamemode_1 (+ (Variables|/Game/Labwork1/Gamemode1.Gamemode1_C|GetGolds _as_gamemode_1) (Variables|Default|GetValue))))
  (Development|PrintString (Utilities|String|Append "You have" (Utilities|String|ToString(Integer) _output_get) "golds"))
  (Actor|DestroyActor))

(fn ConstructionScript)